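; BP_BuildLevelSceneUI is an in-world UI actor for the level builder, holding character, landmark, utility and delete widgets.
; All widgets start collapsed, and each tick it moves to the actor given through SetEditActor.
; The delete widget shows whenever any build widget is visible.
; Its OnDelete event detaches the target's tips via GM_BuildLevel, destroys the target and collapses all widgets.
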(event Custom|OnDelete
  (Utilities|FlowControl|Sequence
    (:then_0
      (Utilities|IsValid (Variables|Default|GetFollow)
        (:Is%20Valid
          (bind _asgm_build_level (Utilities|Casting|CastToGM_BuildLevel (Game|GetGameMode)))
          (Class|ProjectJBuildLevelGameMode|DetachTips _asgm_build_level (Variables|Default|GetFollow))
          (Actor|DestroyActor (Variables|Default|GetFollow))
          (Variables|Default|SetFollow 0))))
    (:then_1
      (Widget|SetVisibility (UserInterface|GetWidget (Variables|Default|GetBuildCharacterWidget)) "Collapsed"))))

(event EventBeginPlay
  (Widget|SetVisibility (UserInterface|GetWidget (Variables|Default|GetBuildCharacterWidget)) "Collapsed")
  (bind _asewbp_delete_point (Utilities|Casting|CastToEWBP_DeletePoint (UserInterface|GetWidget (Variables|Default|GetDeleteWidget))))
  (EventDispatchers|BindEventtoOnClicked (Variables|/Game/EditorBlueprints/UI/BuildLevel/EWBP_DeletePoint.EWBP_DeletePoint_C|GetDeleteBtn _asewbp_delete_point) (EventDispatchers|CreateEvent :!event Custom|OnDelete)))

(event Collision|EventActorBeginOverlap
  (params (OtherActor :type Actor%20Object%20Reference)))

(event EventTick
  (params (DeltaSeconds :type Float%20%28single-precision%29))
  (bind _follow (Variables|Default|GetFollow))
  (Utilities|FlowControl|Sequence
    (:then_0
      (Utilities|IsValid _follow
        (:Is%20Valid
          (Transformation|SetActorLocation (Transformation|GetActorLocation _follow) false false))))
    (:then_1
      (if (Math|Boolean|ORBoolean (Widget|IsVisible (UserInterface|GetWidget (Variables|Default|GetBuildCharacterWidget))) (Widget|IsVisible (UserInterface|GetWidget (Variables|Default|GetBuildLandmarkWidget))) (Widget|IsVisible (UserInterface|GetWidget (Variables|Default|GetBuildUtilityWidget))))
        (Widget|SetVisibility (UserInterface|GetWidget (Variables|Default|GetDeleteWidget)) "Visible")
        (else
          (Widget|SetVisibility (UserInterface|GetWidget (Variables|Default|GetDeleteWidget)) "Collapsed"))))))

(fn ConstructionScript)

(fn SetEditActor
  (params (NewParam :type Actor%20Object%20Reference))
  (Variables|Default|SetFollow NewParam))