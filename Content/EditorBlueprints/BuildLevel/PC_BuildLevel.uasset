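; Player controller for the build-level editor, which shows the matching editing UI for a selected card or actor.
; On BeginPlay it locks the mouse in game-and-UI input, disables UI navigation and caches the BP_BuildLevelSceneUI actor.
; EditCard passes the actor to that UI, then toggles its widgets: character or landmark by card type, or nav point when the card interface is absent.
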(event EventBeginPlay
  (bind _self self)
  (Input|SetInputModeGameOnly _self false)
  (Input|SetInputModeGameandUI _self 0 "LockAlways" false false)
  (Class|ProjectJBlueprintFunctionLibrary|DisableUINav)
  (bind _returnvalue (Actor|GetActorOfClass "/Game/EditorBlueprints/BP_BuildLevelSceneUI.BP_BuildLevelSceneUI_C"))
  (Variables|Default|SetSceneUIActor _returnvalue))

(event EventTick
  (params (DeltaSeconds :type Float%20%28single-precision%29)))

(event EventEditCard
  (params (Actor :type Actor%20Object%20Reference))
  (Utilities|FlowControl|Sequence
    (:then_0
      (Default|SetEditActor (Variables|Default|GetSceneUIActor) Actor))
    (:then_1
      (if (Utilities|DoesObjectImplementInterface Actor "/Script/ProjectJ.ProjectJCardInterface")
        (bind _returnvalue (Class|ProjectJCardInterface|GetCardType(Message) Actor))
        (switch Utilities|FlowControl|Switch|SwitchonEProjectJCardType _returnvalue
          (:Character
            (Widget|SetVisibility (UserInterface|GetWidget (Variables|/Game/EditorBlueprints/BP_BuildLevelSceneUI.BP_BuildLevelSceneUI_C|GetBuildCharacterWidget (Variables|Default|GetSceneUIActor))) "Visible")
            (Widget|SetVisibility (UserInterface|GetWidget (Variables|/Game/EditorBlueprints/BP_BuildLevelSceneUI.BP_BuildLevelSceneUI_C|GetBuildNavPointWidget (Variables|Default|GetSceneUIActor))) "Collapsed")
            (Widget|SetVisibility (UserInterface|GetWidget (Variables|/Game/EditorBlueprints/BP_BuildLevelSceneUI.BP_BuildLevelSceneUI_C|GetBuildLandmarkWidget (Variables|Default|GetSceneUIActor))) "Collapsed"))
          (:Landmark
            (Widget|SetVisibility (UserInterface|GetWidget (Variables|/Game/EditorBlueprints/BP_BuildLevelSceneUI.BP_BuildLevelSceneUI_C|GetBuildLandmarkWidget (Variables|Default|GetSceneUIActor))) "Visible")
            (Widget|SetVisibility (UserInterface|GetWidget (Variables|/Game/EditorBlueprints/BP_BuildLevelSceneUI.BP_BuildLevelSceneUI_C|GetBuildCharacterWidget (Variables|Default|GetSceneUIActor))) "Collapsed")
            (Widget|SetVisibility (UserInterface|GetWidget (Variables|/Game/EditorBlueprints/BP_BuildLevelSceneUI.BP_BuildLevelSceneUI_C|GetBuildNavPointWidget (Variables|Default|GetSceneUIActor))) "Collapsed")))
        (else
          (Widget|SetVisibility (UserInterface|GetWidget (Variables|/Game/EditorBlueprints/BP_BuildLevelSceneUI.BP_BuildLevelSceneUI_C|GetBuildLandmarkWidget (Variables|Default|GetSceneUIActor))) "Collapsed")
          (Widget|SetVisibility (UserInterface|GetWidget (Variables|/Game/EditorBlueprints/BP_BuildLevelSceneUI.BP_BuildLevelSceneUI_C|GetBuildCharacterWidget (Variables|Default|GetSceneUIActor))) "Collapsed")
          (Widget|SetVisibility (UserInterface|GetWidget (Variables|/Game/EditorBlueprints/BP_BuildLevelSceneUI.BP_BuildLevelSceneUI_C|GetBuildNavPointWidget (Variables|Default|GetSceneUIActor))) "Visible"))))))

(fn ConstructionScript)