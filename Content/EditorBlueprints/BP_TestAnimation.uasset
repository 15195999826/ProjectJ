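; BP_TestAnimation is a test Blueprint for triggering card animations with debug keys.
; Three key presses call HideCard, ShowCard and PopupCard, each with a fixed duration; the popup targets a point offset horizontally from the actor's location.
; The animation logic is not defined in this graph, and the BeginPlay, overlap, Tick and construction script hold no custom behavior.
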(event EventBeginPlay
  (|CallParentFunction) ; This node is disabled and will not be called.\nDrag off pins to build functionality.
)

(event Collision|EventActorBeginOverlap
  (params (OtherActor :type Actor%20Object%20Reference))
  (|CallParentFunction OtherActor) ; This node is disabled and will not be called.\nDrag off pins to build functionality.
)

(event EventTick
  (params (DeltaSeconds :type Float%20%28single-precision%29))
  (|CallParentFunction DeltaSeconds) ; This node is disabled and will not be called.\nDrag off pins to build functionality.
)

(event Input|KeyboardEvents|DebugKey3
  (params (Key :type Key%20Structure :default "None") (ActionValue :type Input%20Action%20Value%20Structure))
  (:Pressed
    (Class|ProjectJCardBase|PopupCard (Transformation|GetActorLocation) (+ (Transformation|GetActorLocation) "200.000000,200.000000,0.000000") 0.8)))

(event Input|KeyboardEvents|DebugKey1
  (params (Key :type Key%20Structure :default "None") (ActionValue :type Input%20Action%20Value%20Structure))
  (:Pressed
    (Class|ProjectJCardBase|HideCard 0.5)))

(event Input|KeyboardEvents|DebugKey2
  (params (Key :type Key%20Structure :default "None") (ActionValue :type Input%20Action%20Value%20Structure))
  (:Pressed
    (Class|ProjectJCardBase|ShowCard 0.5)))

(fn ConstructionScript
  (|CallParentFunction))