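; BP_PerformManager presents story records to the player through a modal story widget.
; It overrides PerformStory, calls the parent, then rebuilds a string list from the record's story entries.
; It asynchronously shows WBP_Story_Modal, passes it that list to start the story, and calls PerformStoryEnd when the modal closes.
; PerformStoryEnd only forwards to the parent implementation.
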(event EventBeginPlay)

(event Collision|EventActorBeginOverlap
  (params (OtherActor :type Actor%20Object%20Reference)))

(event EventTick
  (params (DeltaSeconds :type Float%20%28single-precision%29)))

(event EventPerformStory
  (params (InStoryRecord :type Project%20J%20Story%20Record%20Structure%20%28by%20ref%29))
  (|CallParentFunction InStoryRecord)
  (Utilities|FlowControl|Sequence
    (:then_0
      (Utilities|Array|Clear (Variables|Default|GetIn%20Context))
      (for _array_element (Utilities|Struct|BreakProjectJStoryRecord InStoryRecord)
        (Utilities|Array|Add (Variables|Default|GetIn%20Context) (Utilities|String|ToString(Text) _array_element))))
    (:then_1
      (bind _userwidget (|AsyncShowModalfromClass "/Game/Blueprints/UI/Modal/WBP_Story_Modal.WBP_Story_Modal_C")
        (:then
          (bind _aswbp_story_modal (Utilities|Casting|CastToWBP_Story_Modal _userwidget))
          (Default|StartStory _aswbp_story_modal (Variables|Default|GetIn%20Context)))
        (:OnClose
          (Class|ProjectJPerformManager|PerformStoryEnd))))))

(event EventPerformStoryEnd
  (|CallParentFunction))

(fn ConstructionScript)