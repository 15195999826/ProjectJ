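; PC_ProjectJ_Main is a player controller that sets up input and the opening camera view.
; On BeginPlay it ends in Game and UI input mode with a locked mouse, disables UI navigation, and views through the first CameraActor tagged "StartMenu".
; Debug keys print a localized test string and toggle BP_SpringArmCamera between perspective and orthographic projection.
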(event EventBeginPlay
  (bind _self self)
  (Input|SetInputModeGameOnly _self false)
  (Input|SetInputModeGameandUI _self 0 "LockAlways" false false)
  (Class|ProjectJBlueprintFunctionLibrary|DisableUINav)
  (bind _outactors (Actor|GetAllActorsOfClass "/Script/Engine.CameraActor"))
  (bind _array_element (Utilities|Array|ForEachLoopwithBreak _outactors :!label _label)
    (:LoopBody
      (if (Actor|ActorHasTag _array_element "StartMenu")
        (Game|Player|SetViewTargetwithBlend _array_element 0.0 "VTBlend_Linear" 0.0 false)
        (goto _label Break)))))

(event EventTick
  (params (DeltaSeconds :type Float%20%28single-precision%29)))

(event Input|KeyboardEvents|DebugKey1
  (params (Key :type Key%20Structure :default "None") (ActionValue :type Input%20Action%20Value%20Structure))
  (:Pressed
    (bind _returnvalue (Class|ProjectJBlueprintFunctionLibrary|GetLocText "" "Hello" (Utilities|Text|FormatText "测试")))
    (Development|PrintText _returnvalue)))

(event Input|KeyboardEvents|DebugKeyTab
  (params (Key :type Key%20Structure :default "None") (ActionValue :type Input%20Action%20Value%20Structure))
  (:Pressed
    (bind _returnvalue (Actor|GetActorOfClass "/Game/Blueprints/BP_SpringArmCamera.BP_SpringArmCamera_C"))
    (if (Utilities|Enum|Equal(Enum) (Variables|/Script/Engine.CameraComponent|GetProjectionMode (Variables|/Script/Engine.CameraActor|GetCameraComponent _returnvalue)) "Perspective")
      (Default|ChangetoOrt _returnvalue)
      (else
        (Default|ChangetoPerspective _returnvalue)))))

(fn ConstructionScript)