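; BP_SceneUI is a dialogue actor that steps through Context lines on a WBP_Talk widget component after StartTalkwith receives a card.
; Clicking the widget, which relies on world-space UI for click events, reveals the full line or starts the next.
; The widget's OnComplete advances the index.
; Collision is enabled only during dialogue; a click after the last line hides the widget, disables collision and calls OnTalkOver.
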(event OnClicked(TalkWidgetComponent)
  (params (TouchedComponent :type Primitive%20Component%20Object%20Reference) (ButtonPressed :type Key%20Structure :default "None"))
  ;[1 0.1354 0.1453] 踩坑， World UI才存在点击事件
  (if (Variables|Default|GetIsTalking)
    (Default|ShowFullContent (Variables|Default|GetAs%20WBP%20Talk))
    (elif (>= (Variables|Default|GetIndex) (Utilities|Array|Length (Variables|Default|GetContext)))
      (Rendering|SetVisibility (Variables|Default|GetTalkWidgetComponent) false false)
      (Collision|SetActorEnableCollision false)
      (Default|CallOnTalkOver)
      (else
        (CallFunction|StartTalk)))))

(event Custom|OnComplete_Event
  (Variables|Default|SetIsTalking false)
  (Math|Integer|IncrementInt (Variables|Default|GetIndex)))

(event Custom|Start%20Talk
  (Variables|Default|SetIsTalking true)
  (Default|StartTalk (Variables|Default|GetAs%20WBP%20Talk) (Utilities|Array|Get(acopy) (Variables|Default|GetContext) (Variables|Default|GetIndex))))

(event EventBeginPlay
  (Collision|SetActorEnableCollision false)
  (bind _aswbp_talk (Utilities|Casting|CastToWBP_Talk (UserInterface|GetWidget (Variables|Default|GetTalkWidgetComponent))))
  (bind _output_get (Variables|Default|SetAs%20WBP%20Talk _aswbp_talk))
  (EventDispatchers|BindEventtoOnComplete _output_get (delegate Custom|OnComplete_Event)))

(event Collision|EventActorBeginOverlap
  (params (OtherActor :type Actor%20Object%20Reference)))

(event EventTick
  (params (DeltaSeconds :type Float%20%28single-precision%29)))

(event EventStartTalkwith
  (params (InCard :type Project%20J%20Card%20Base%20Object%20Reference))
  (|CallParentFunction InCard)
  (Collision|SetActorEnableCollision true)
  (Variables|Default|SetIndex 0)
  (CallFunction|StartTalk))

(fn ConstructionScript)