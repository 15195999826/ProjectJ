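; Blueprint function library of shared helpers for Project J, covering build-level tip labels, game instance access and UI creation.
; UpdateBuildLevelTips writes a row name into the TextRender of an attached BP_BuildLevelTips actor, printing a debug message when none is found.
; GetBPProjectJInstance returns the game instance cast to BP_ProjectJGameInstance.
; PushUIClass creates a widget from a class, passes it to PushUI with overlay and alignment settings, and returns it.
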(fn UpdateBuildLevelTips
  (params (InActor :type Actor%20Object%20Reference) (InRowName :type Name))
  (LocalVariables|SetFindTips false)
  (bind _array_element (Utilities|Array|ForEachLoopwithBreak (Actor|GetAttachedActors InActor true false) :!label _label)
    (:LoopBody
      (bind _asbp_build_level_tips (Utilities|Casting|CastToBP_BuildLevelTips _array_element))
      (LocalVariables|SetTips _asbp_build_level_tips)
      (LocalVariables|SetFindTips true)
      (goto _label Break))
    (:Completed
      (if (LocalVariables|GetFindTips)
        (Rendering|Components|TextRender|SetText (Variables|/Script/ProjectJ.ProjectJBuildLevelTipsActor|GetTextRenderComponent (LocalVariables|GetTips)) (Utilities|Text|ToText(Name) InRowName))
        (else
          (Development|PrintString 0 "没有对应的Tips" true true "(R=1.000000,G=0.169616,B=0.089927,A=1.000000)"))))))

(fn GetBPProjectJInstance
  (bind _asbp_project_jgame_instance (Utilities|Casting|CastToBP_ProjectJGameInstance (Game|GetGameInstance))
    (:then
      (return _asbp_project_jgame_instance))
    (:CastFailed
      (return 0))))

(fn PushUIClass
  (params (Overlay :type EProjectJUIOverlayType%20Enum :default "BackEnd") (WidgetClass :type User%20Widget%20Class%20Reference) (HorizontalAlignment :type EHorizontalAlignment%20Enum :default "HAlign_Fill") (VerticalAlignment :type EVerticalAlignment%20Enum :default "VAlign_Fill"))
  (bind _returnvalue (UserInterface|CreateWidget WidgetClass))
  (bind _output_get (LocalVariables|SetNewWidget _returnvalue))
  (Class|ProjectJBlueprintFunctionLibrary|PushUI (LocalVariables|Get__WorldContext) Overlay _output_get HorizontalAlignment VerticalAlignment)
  (return (LocalVariables|GetNewWidget)))