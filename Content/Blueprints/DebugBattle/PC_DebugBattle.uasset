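; Debug battle player controller that opens the debug battle main widget with game-and-UI input and provides hotkeys for testing the poison gameplay effect.
; DebugKey1 applies poison to the BP_Character found in the world, choosing its round value from the current poison stack count.
; DebugKey2 removes one stack through the effect handle cached by the last application.
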(event EventBeginPlay
  (bind _self self)
  (Input|SetInputModeGameOnly _self false)
  (Input|SetInputModeGameandUI _self 0 "LockAlways" false false)
  (Class|ProjectJBlueprintFunctionLibrary|DisableUINav)
  (bind _returnvalue (UserInterface|CreateWidget "/Game/Blueprints/DebugBattle/UI/DebugBattle_WBP_Main.DebugBattle_WBP_Main_C"))
  (UserInterface|Viewport|AddtoViewport _returnvalue 0))

(event EventTick
  (params (DeltaSeconds :type Float%20%28single-precision%29)))

(event Input|KeyboardEvents|DebugKey2
  (params (Key :type Key%20Structure :default "None") (ActionValue :type Input%20Action%20Value%20Structure))
  (:Pressed
    (bind _returnvalue (Actor|GetActorOfClass "/Game/Blueprints/Card/BP_Character.BP_Character_C"))
    (GameplayEffects|RemoveActiveGameplayEffect (Ability|GetAbilitySystemComponent _returnvalue) (Variables|Default|GetCachedTestGEHandle) 1)))

(event Input|KeyboardEvents|DebugKey3
  (params (Key :type Key%20Structure :default "None") (ActionValue :type Input%20Action%20Value%20Structure)))

(event Input|KeyboardEvents|DebugKey1
  (params (Key :type Key%20Structure :default "None") (ActionValue :type Input%20Action%20Value%20Structure))
  (:Pressed
    (bind _returnvalue (Actor|GetActorOfClass "/Game/Blueprints/Card/BP_Character.BP_Character_C"))
    (Utilities|FlowControl|Sequence
      (:then_0
        (bind _returnvalue_2 (Class|AbilitySystemComponent|GetActiveEffects (Ability|GetAbilitySystemComponent _returnvalue) (Utilities|Struct|MakeGameplayEffectQuery "(null).None" "(TokenStreamVersion=0,TagDictionary=((TagName=\"Feature.Poison\")),QueryTokenStream=(0,1,2,1,0),UserDescription=\"\",AutoDescription=\" ALL( Feature.Poison )\")")))
        (if (>= (Utilities|Array|Length _returnvalue_2) 1)
          (bind _returnvalue_3 (Ability|GameplayEffect|GetActiveGameplayEffectStackCount (Utilities|Array|Get(acopy) _returnvalue_2)))
          (if (>= _returnvalue_3 2)
            (Variables|Default|SetTempRound 2)
            (else
              (Variables|Default|SetTempRound -1)))
          (else
            (Variables|Default|SetTempRound -1))))
      (:then_1
        (bind _returnvalue_4 (Class|ProjectJGameBFL|SimpleApplyGEtoSelf _returnvalue "/Game/Blueprints/GAS/GE/Features/Feature_Poision.Feature_Poision_C" 1.0 (Variables|Default|GetTempRound)))
        (Variables|Default|SetCachedTestGEHandle _returnvalue_4)))))

(fn ConstructionScript)